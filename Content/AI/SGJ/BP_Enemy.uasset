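; AI enemy character with a stat widget, data-driven melee and ranged attacks, and an arced wall jump.
; Tick sets turn flags from controller-versus-actor yaw and copies BaseStatComponent HP to the Blackboard, where Active also sets a flag.
; DT_SkillData rows drive attacks: melee runs timed socket-to-socket box traces dealing fixed damage, while ranged spawns a Bullet toward Target.
; WallJump pauses movement, then launches the character along a suggested projectile arc scaled by a booster.
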(event `self.ReceiveBeginPlay`
  (set `self.AIControllerClass` "/Game/AI/SGJ/AIC_EnemyController.AIC_EnemyController_C")
  (`|ExecutionSequence`
    (:`then_0`
      (bind _outrownames (`DataTableFunctionLibrary.GetDataTableRowNames` "/Game/AI/SGJ/DT_AI_Skill.DT_AI_Skill"))
      (set `self.Out Row Names` _outrownames))
    (:`then_1`
      (bind _returnvalue (`|CreateWidget` "/Game/yjs/WBP_StatWidget.WBP_StatWidget_C"))
      (set `/Game/yjs/WBP_StatWidget.ownerActor` self _returnvalue)
      (`WidgetComponent.SetWidget` (`self.Widget`) _returnvalue))))

(event `self.ReceiveTick`
  (params (DeltaSeconds :type "Float (single-precision)"))
  (bind (_returnvalue_roll _returnvalue_pitch _returnvalue_yaw) (`KismetMathLibrary.BreakRotator` (`KismetMathLibrary.NormalizedDeltaRotator` (`self.K2_GetActorRotation` (`self.GetController`)) (`self.K2_GetActorRotation`))))
  (`|ExecutionSequence`
    (:`then_0`
      (if (`KismetMathLibrary.InRange_FloatFloat` _returnvalue_yaw -0.1 0.1)
        (if (> _returnvalue_yaw 0.0)
          (set `self.TurnRight` true)
          (else
            (set `self.TurnLeft` true)))
        (else
          (set `self.TurnRight` false)
          (set `self.TurnLeft` false))))
    (:`then_1`
      (`BlackboardComponent.SetValueAsFloat` (`AIBlueprintHelperLibrary.GetBlackboard` (`self.GetController`)) (`self.HealthPoint`) (`BaseStatComponent.hp` (`self.GetComponentByClass` self "/Script/BaseModule.BaseStatComponent"))))))

(event `WallJump`
  (params (Agent :type "Actor Object Reference") (Destination :type "Vector Structure") (JumpBooster :type "Float (double-precision)"))
  (bind _tempspeed (`self.tempSpeed`))
  (bind _charactermovement (`self.CharacterMovement`))
  (bind _output_get (set `self.As캐릭터` self))
  (set `self.tempSpeed` (`self.moveSpeed`))
  (set `self.moveSpeed` 0.0)
  (set `CharacterMovementComponent.MaxWalkSpeed` 0.0 _charactermovement)
  (set `self.Is Jump` true)
  (`KismetSystemLibrary.Delay` 0.6)
  (bind _outlaunchvelocity (`GameplayStatics.SuggestProjectileVelocity_CustomArc` (`self.K2_GetActorLocation` _output_get) Destination))
  (`KismetSystemLibrary.Delay` 0.1)
  (set `CharacterMovementComponent.MaxWalkSpeed` _tempspeed _charactermovement)
  (set `self.moveSpeed` _tempspeed)
  (`self.LaunchCharacter` (`self.As캐릭터`) (* _outlaunchvelocity JumpBooster) true true)
  (set `self.Is Jump` false))

(event `StartMeleeAttack`
  (params (RightChk :type Boolean) (RowName :type Name))
  (bind _returnvalue (`|GetDataTableRow` "/Game/AI/Public_Space/AI_Behavior/BP/AI_Data/DT_SkillData.DT_SkillData" RowName)
    (:`then`
      (bind (_rightchk _attackanim _attacktype _attack_melee_parts_start _attack_melee_parts_end _attack_size _attack_delaytime _attack_loop) (break `/Game/AI/Public_Space/AI_Behavior/BP/AI_Data/F_SkillData` _returnvalue))
      (set `self.Attack_Motion` _attackanim)
      (bind _returnvalue_2 (`KismetSystemLibrary.K2_SetTimerDelegate` (delegate `AttackTrace`) _attack_delaytime _attack_loop))
      (set `self.AttackTimeHandle` _returnvalue_2))))

(event `AttackTrace`
  (`self.EnemyBaseAttack` (stale `StartMeleeAttack` RowName)))

(event `StopMeleeAttack`
  (`KismetSystemLibrary.K2_ClearAndInvalidateTimerHandle` (`self.AttackTimeHandle`)))

(event `ShootAttack`
  (params (RowName :type Name))
  (bind _returnvalue (`|GetDataTableRow` "/Game/AI/Public_Space/AI_Behavior/BP/AI_Data/DT_SkillData.DT_SkillData" RowName)
    (:`then`
      (`self.EnemyBaseAttack` RowName)
      (set `self.Attack_Motion` (`.AttackAnim_5_FA7E5C914B0BDD409D7A63B6B085AAE5` (break `/Game/AI/Public_Space/AI_Behavior/BP/AI_Data/F_SkillData` _returnvalue))))))

(event `Active`
  (`BlackboardComponent.SetValueAsBool` (`AIBlueprintHelperLibrary.GetBlackboard` (`self.GetController`)) (`self.ActiveClass`) true))

(fn `EnemyBaseAttack`
  (params (RowName :type Name))
  (bind _returnvalue (`self.K2_GetActorLocation` self))
  (bind _returnvalue_2 (`|GetDataTableRow` "/Game/AI/Public_Space/AI_Behavior/BP/AI_Data/DT_SkillData.DT_SkillData" RowName)
    (:`then`
      (switch `/Game/AI/Public_Space/AI_Behavior/BP/AI_Data/E_AttackType` (`.AttackType_8_37551CB74D23E98E0605C990A619DF78` (break `/Game/AI/Public_Space/AI_Behavior/BP/AI_Data/F_SkillData` _returnvalue_2))
        (:`NewEnumerator0`
          (bind _outhit (`KismetSystemLibrary.BoxTraceSingle` :`Start` (`SceneComponent.GetSocketLocation` (`self.Mesh`) (`.Attack_Melee_Parts_Start_14_56A76D7144A568AA9F166CAEBB6C04CC` (break `/Game/AI/Public_Space/AI_Behavior/BP/AI_Data/F_SkillData` _returnvalue_2))) :`End` (`SceneComponent.GetSocketLocation` (`self.Mesh`) (`.Attack_Melee_Parts_End_16_150E280641EAAA2EF1FBDEB8890FBB89` (break `/Game/AI/Public_Space/AI_Behavior/BP/AI_Data/F_SkillData` _returnvalue_2))) :`HalfSize` (`.Attack_Size_19_667EE41E442729F4BEEEAA8F7AC136C4` (break `/Game/AI/Public_Space/AI_Behavior/BP/AI_Data/F_SkillData` _returnvalue_2)) :`TraceChannel` "TraceTypeQuery1" :`DrawDebugType` "ForDuration" :`DrawTime` 0.2))
          (bind (_bblockinghit _binitialoverlap _time _distance _location _impactpoint _normal _impactnormal _physmat _hitactor) (`GameplayStatics.BreakHitResult` _outhit))
          (`KismetSystemLibrary.PrintString` (`KismetSystemLibrary.GetDisplayName` _hitactor))
          (`/Engine/EditorBlueprintResources/StandardMacros.IsValid` _hitactor
            (:`Is Valid`
              (bind _returnvalue_3 (`self.GetComponentByClass` _hitactor "/Script/BaseModule.BaseStatComponent"))
              (if (`KismetSystemLibrary.IsValid` _returnvalue_3)
                (`KismetSystemLibrary.K2_ClearAndInvalidateTimerHandle` (`self.AttackTimeHandle`))
                (`BaseStatComponent.Attacked` _returnvalue_3 10.0)))))
        (:`NewEnumerator1`
          (bind _returnvalue_4 (`|SpawnActorFromClass` "/Game/AI/Public_Space/BP/Weapon/Bullet/Bullet.Bullet_C" (`KismetMathLibrary.MakeTransform` _returnvalue (`KismetMathLibrary.Conv_VectorToRotator` (`KismetMathLibrary.Normal` (- (`self.K2_GetActorLocation` (`self.target`)) _returnvalue))) (`.Attack_Size_19_667EE41E442729F4BEEEAA8F7AC136C4` (break `/Game/AI/Public_Space/AI_Behavior/BP/AI_Data/F_SkillData` _returnvalue_2))) "Undefined" "MultiplyWithRoot" null null))
          (set `ProjectileMovementComponent.InitialSpeed` (`.Attack_Speed_28_11A2FDEA4D31159F0D0B3496EEB35B57` (break `/Game/AI/Public_Space/AI_Behavior/BP/AI_Data/F_SkillData` _returnvalue_2)) (`/Game/AI/Public_Space/BP/Weapon/Bullet/Bullet.ProjectileMovement` _returnvalue_4))
          (`self.StopMeleeAttack`))))))

(fn `UserConstructionScript`)