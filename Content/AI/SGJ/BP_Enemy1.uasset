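; BP_Enemy1 is an enemy character Blueprint with an overhead-style stat widget, a wall jump and AI activation.
; BeginPlay creates WBP_StatWidget, sets itself as owner and assigns it to the widget component.
; WallJump halts movement and flags IsJump during a short wind-up, then restores speed and launches along a suggested projectile arc scaled by JumpBooster.
; Active sets a blackboard bool on its controller; EnemyBaseAttack is empty.
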(event `self.ReceiveBeginPlay`
  (`|ExecutionSequence`
    (:`then_1`
      (bind _returnvalue (`|CreateWidget` "/Game/yjs/WBP_StatWidget.WBP_StatWidget_C"))
      (set `/Game/yjs/WBP_StatWidget.ownerActor` self _returnvalue)
      (`WidgetComponent.SetWidget` (`self.Widget`) _returnvalue))))

(event `self.ReceiveTick`
  (params (DeltaSeconds :type "Float (single-precision)")))

(event `WallJump`
  (params (Agent :type "Actor Object Reference") (Destination :type "Vector Structure") (JumpBooster :type "Float (double-precision)"))
  (bind _tempspeed (`self.tempSpeed`))
  (bind _charactermovement (`self.CharacterMovement`))
  (bind _output_get (set `self.As캐릭터` self))
  (set `self.tempSpeed` (`self.moveSpeed`))
  (set `self.moveSpeed` 0.0)
  (set `CharacterMovementComponent.MaxWalkSpeed` 0.0 _charactermovement)
  (set `self.Is Jump` true)
  (`KismetSystemLibrary.Delay` 0.6)
  (bind _outlaunchvelocity (`GameplayStatics.SuggestProjectileVelocity_CustomArc` (`self.K2_GetActorLocation` _output_get) Destination))
  (`KismetSystemLibrary.Delay` 0.1)
  (set `CharacterMovementComponent.MaxWalkSpeed` _tempspeed _charactermovement)
  (set `self.moveSpeed` _tempspeed)
  (`self.LaunchCharacter` (`self.As캐릭터`) (* _outlaunchvelocity JumpBooster) true true)
  (set `self.Is Jump` false))

(event `Active`
  (`BlackboardComponent.SetValueAsBool` (`AIBlueprintHelperLibrary.GetBlackboard` (`self.GetController`)) (`self.ActiveClass`) true))

(fn `EnemyBaseAttack`
  (params (RowName :type Name)))

(fn `UserConstructionScript`)