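; BP_NavJump is a nav link actor that makes enemies jump when they reach its smart link.
; On SmartLinkReached, it casts the agent to BP_Enemy and calls WallJump with the link destination and its JumpBoost multiplier, leaving the jump itself to the enemy.
; An unconnected older chain remains, which paused movement, computed a projectile arc velocity and launched the character directly.
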(event `self.ReceiveSmartLinkReached`
  (params (Agent :type "Actor Object Reference") (Destination :type "Vector Structure (by ref)"))
  (bind _asbp_enemy (cast `/Game/AI/SGJ/BP_Enemy` Agent))
  (`/Game/AI/SGJ/BP_Enemy.WallJump` _asbp_enemy null Destination (`self.jumpBoost`)))

(fn `UserConstructionScript`)