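; Demo actor for a Niagara dash effect: a skeletal mesh runs along a spline when E or V is pressed.
; A timeline moves and rotates the mesh along the spline while an attached Niagara system plays, then deactivates the effects and returns to idle.
; A box trigger enables input only while the ThirdPersonCharacter overlaps it.
; The construction script applies a fresnel material and pushes one color to the mesh and hand effects.
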(event `Key|E`
  (params (Key :type "Key Structure"))
  (bind _spline (`self.Spline`))
  (:`Pressed`
    (set `self.Condition` false)
    (if (not (`self.Condition`)) :!label _label
      (set `self.Condition` true)
      (`SkeletalMeshComponent.PlayAnimation` (`self.SkeletalMesh`) "/Game/AI/AUS/NiagaraDashEffects/Demo/Mannequin/Animations/ThirdPersonRun.ThirdPersonRun" true)
      (`|ExecutionSequence`
        (:`then_0`
          (bind (_direction _float) (`Timeline|Turn Time`)
            (:`Update`
              (bind _returnvalue (* (`SplineComponent.GetSplineLength` _spline) _float))
              (bind (_returnvalue_roll _returnvalue_pitch _returnvalue_yaw) (`KismetMathLibrary.BreakRotator` (`SplineComponent.GetRotationAtDistanceAlongSpline` _spline _returnvalue "Local")))
              (`SceneComponent.K2_SetWorldTransform` (`self.SkeletalMesh`) (`KismetMathLibrary.MakeTransform` (`SplineComponent.GetLocationAtDistanceAlongSpline` _spline _returnvalue "World") (`KismetMathLibrary.MakeRotator` _returnvalue_roll _returnvalue_pitch (+ _returnvalue_yaw -90.0))) false false))
            (:`Finished`
              (`ActorComponent.Deactivate` (stale _returnvalue_2))
              (`ActorComponent.Deactivate` (`self.NS_HandP`))
              (`ActorComponent.Deactivate` (`self.NS_HandP1`))
              (`SkeletalMeshComponent.PlayAnimation` (`self.SkeletalMesh`) "/Game/AI/AUS/NiagaraDashEffects/Demo/Mannequin/Animations/ThirdPersonIdle.ThirdPersonIdle" true))))
        (:`then_1`
          (bind _returnvalue_2 (`NiagaraFunctionLibrary.SpawnSystemAttached` (`self.System Template`) (`self.SkeletalMesh`) "None" (0.0 0.0 0.0) (struct) "KeepRelativeOffset")))))))

(event `Key|V`
  (params (Key :type "Key Structure"))
  (:`Pressed`
    (set `self.Condition` false)
    (goto _label)))

(event `self.Box.OnComponentBeginOverlap`
  (params (OverlappedComponent :type "PrimitiveComponent Object Reference") (OtherActor :type "Actor Object Reference") (OtherComp :type "PrimitiveComponent Object Reference") (OtherBodyIndex :type Integer) (bFromSweep :type Boolean) (SweepResult :type "HitResult Structure (by ref)"))
  (cast `/Game/AI/AUS/NiagaraDashEffects/Demo/ThirdPersonBP/Blueprints/ThirdPersonCharacter` OtherActor)
  (`self.EnableInput` (`GameplayStatics.GetPlayerController` 0)))

(event `self.Box.OnComponentEndOverlap`
  (params (OverlappedComponent :type "PrimitiveComponent Object Reference") (OtherActor :type "Actor Object Reference") (OtherComp :type "PrimitiveComponent Object Reference") (OtherBodyIndex :type Integer))
  (cast `/Game/AI/AUS/NiagaraDashEffects/Demo/ThirdPersonBP/Blueprints/ThirdPersonCharacter` OtherActor)
  (`self.DisableInput` (`GameplayStatics.GetPlayerController` 0)))

(fn `UserConstructionScript`
  (bind _skeletalmesh (`self.SkeletalMesh`))
  (`|ExecutionSequence`
    (:`then_0`
      (for (_ _array_index) (`MeshComponent.GetMaterials` _skeletalmesh)
        (`PrimitiveComponent.SetMaterial` _skeletalmesh _array_index "/Game/AI/AUS/NiagaraDashEffects/Demo/Mannequin/Character/Materials/MI_UE4Man_BodyFres.MI_UE4Man_BodyFres")
        (`MeshComponent.SetVectorParameterValueOnMaterials` _skeletalmesh "Fresnel Color (V3)" (`KismetMathLibrary.Conv_LinearColorToVector` (`self.Color`)))
        (`MeshComponent.SetScalarParameterValueOnMaterials` _skeletalmesh "Lava (S)" (`self.Parameter Value`))))
    (:`then_1`
      (`NiagaraComponent.SetVariableLinearColor` (`self.NS_HandP`) "Color" (`self.Color`))
      (`NiagaraComponent.SetVariableLinearColor` (`self.NS_HandP1`) "Color" (`self.Color`)))))