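; Effect spawner actor that plays a chosen particle system when placed or spawned.
; On BeginPlay it assigns the Fx template, activates it and waits Interval, then reactivates it if IsLoop is set or destroys itself otherwise.
; The construction script optionally tints the effect by writing Color and ColorSub into the "color" and "color2" vector parameters.
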(event `self.ReceiveBeginPlay`
  ;[1 1 1] fx activate
  (`ParticleSystemComponent.SetTemplate` (`self.ParticleSystem`) (`self.fx`))
  (`ActorComponent.Activate` (`self.ParticleSystem`) true :!label _label)
  ;[1 1 1] loop control
  (`KismetSystemLibrary.Delay` (`self.interval`))
  (if (`self.isLoop`)
    (goto _label)
    (else
      ;[1 1 1] destroy
      (`self.K2_DestroyActor`))))

(fn `UserConstructionScript`
  ;[1 1 1] color control
  (if (`self.isChangeColor`)
    (`ParticleSystemComponent.SetVectorParameter` (`self.ParticleSystem`) "color" (`KismetMathLibrary.Conv_LinearColorToVector` (`self.color`)))
    (`ParticleSystemComponent.SetVectorParameter` (`self.ParticleSystem`) "color2" (`KismetMathLibrary.Conv_LinearColorToVector` (`self.colorSub`)))))